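; PG_Wall is a procedural generation Blueprint that builds a grid of repeated mesh pieces, named as a wall.
; Its Construction Script runs nested loops over XValue and YValue, adding an InstancedStaticMesh instance at each cell in local space.
; Cells use fixed, unequal X and Y spacing with zero Z, no rotation and unit scale.
; The Event Graph holds only disabled stub events, so it has no runtime logic.
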(fn `UserConstructionScript`
  (for _index (range (`self.X_Value`))
    (set `self.Looop_X` _index)
    (for _index_2 (range (`self.Y_Value`))
      (set `self.Loop_Y` _index_2)
      (`InstancedStaticMeshComponent.AddInstance` (`self.InstancedStaticMesh`) (`KismetMathLibrary.MakeTransform` (`KismetMathLibrary.MakeVector` (* (`self.Looop_X`) 400.0) (* (`self.Loop_Y`) 200.0))) false))))