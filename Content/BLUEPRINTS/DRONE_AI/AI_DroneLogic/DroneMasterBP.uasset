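; Master drone enemy pawn that patrols waypoints, hunts the player and shoots on sight.
; Looping timers run view-cone and line-trace detection, movement and shooting, switching between Patrolling, Aggro and a last-known-location search.
; Shots use a hitscan trace for damage, plus a projectile actor and a destruction field at impact.
; Head hits kill instantly; death spawns a wreck and updates the player HUD's targets.
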(event `self.ReceiveTick`
  (params (DeltaSeconds :type "Float (single-precision)"))
  (`self.RotatePropellers`))

(event `RotatePropellers`
  (for _array_element (`|MakeArray` (`self.LR-Prop`) (`self.RR-Prop`) (`self.LF-Prop`) (`self.RF-Prop`))
    (`/Engine/EditorBlueprintResources/StandardMacros.IsValid` (`StaticMeshComponent.StaticMesh` _array_element)
      (:`Is Valid`
        (`SceneComponent.K2_AddLocalRotation` _array_element (`KismetMathLibrary.MakeRotator` 0.0 0.0 (* (`GameplayStatics.GetWorldDeltaSeconds`) 2000.0)) false false)))))

(event `CanShoot?`
  (bind _projectilespawnpoint (`self.ProjectileSpawnPoint`))
  (bind _projectilespawnpoint_2 (`self.ProjectileSpawnPoint`))
  (bind _returnvalue (`SceneComponent.K2_GetComponentLocation` (`self.ProjectileSpawnPoint`)))
  (bind _returnvalue_2 (`SceneComponent.K2_GetComponentLocation` _projectilespawnpoint))
  (switch `/Game/BLUEPRINTS/DRONE_AI/AI_DroneLogic/E_FlyModes` (`self.FlyModes`)
    (:`NewEnumerator1`
      (if (> (`KismetMathLibrary.Dot_VectorVector` (`SceneComponent.GetForwardVector` (`self.FowardVector`)) (`KismetMathLibrary.Normal` (- (`self.K2_GetActorLocation` (`GameplayStatics.GetPlayerCharacter` 0)) (`self.K2_GetActorLocation`)))) (`self.ShootDOTproduct`))
        (bind (_outhit _returnvalue_3) (`KismetSystemLibrary.LineTraceSingle` _returnvalue_2 (+ _returnvalue_2 (* (`SceneComponent.GetForwardVector` _projectilespawnpoint) (`self.TurretRange`))) "TraceTypeQuery1" false (`|MakeArray` self :!type "Actor Object Reference")))
        (if _returnvalue_3
          _
          (else
            _))
        (`GameplayStatics.PlaySound2D` "/Game/BLUEPRINTS/Sounds/Interaction/DroneFire_Cue.DroneFire_Cue" 1.0 1.0 0.0 null null)
        (bind (_bblockinghit _binitialoverlap _time _distance _location _impactpoint _normal _impactnormal _physmat _hitactor _hitcomponent _hitbonename _bonename _hititem _elementindex _faceindex _tracestart _traceend) (`GameplayStatics.BreakHitResult` _outhit))
        (if (`KismetSystemLibrary.DoesImplementInterface` _hitactor "/Game/BLUEPRINTS/TakeDamage.TakeDamage_C")
          (message `/Game/BLUEPRINTS/TakeDamage.ITakeDamage` _hitactor _hitbonename 15.0))
        (bind (_returnvalue_location _returnvalue_rotation) (`KismetMathLibrary.BreakTransform` (`KismetMathLibrary.MakeTransform` _returnvalue (`KismetMathLibrary.FindLookAtRotation` _returnvalue (`KismetMathLibrary.SelectVector` _impactpoint _traceend _returnvalue_3)))))
        (`|SpawnActorFromClass` "/Game/BLUEPRINTS/DRONE_AI/AI_DroneLogic/DroneProjectileBP.DroneProjectileBP_C" (`KismetMathLibrary.MakeTransform` _returnvalue_location _returnvalue_rotation) "Undefined" "MultiplyWithRoot" null null)
        (`GameplayStatics.SpawnEmitterAtLocation` "/Game/BLUEPRINTS/ITEM_Pickups/Weapons/SciFiWeapLight/FX/Particles/P_Impact_Metal_Large_Dark.P_Impact_Metal_Large_Dark" _location (struct) (0.7 0.7 0.7))
        (`GameplayStatics.SpawnEmitterAttached` "/Game/BLUEPRINTS/ITEM_Pickups/Weapons/SciFiWeapLight/FX/Particles/P_Pistol_MuzzleFlash_Dark.P_Pistol_MuzzleFlash_Dark" _projectilespawnpoint_2 "None" (`SceneComponent.K2_GetComponentLocation` _projectilespawnpoint_2) (`SceneComponent.K2_GetComponentRotation` _projectilespawnpoint_2) (1.0 1.0 1.0) "KeepWorldPosition")
        (bind (_returnvalue_location_2 _returnvalue_rotation_2) (`KismetMathLibrary.BreakTransform` (`KismetMathLibrary.Conv_VectorToTransform` _impactpoint)))
        (bind _returnvalue_4 (`|SpawnActorFromClass` "/Game/BLUEPRINTS/Interactables/DestructableMesh/DRONE_FS_MasterField.DRONE_FS_MasterField_C" (`KismetMathLibrary.MakeTransform` (+ _returnvalue_location_2 (* _impactnormal (-3.0 -3.0 -3.0))) _returnvalue_rotation_2) "Undefined" "MultiplyWithRoot" null null))
        (set `self.DestructionREF` _returnvalue_4)
        (set `/Game/BLUEPRINTS/Interactables/DestructableMesh/DRONE_FS_MasterField.ActivationType` "NewEnumerator4" (`self.DestructionREF`))
        (set `/Game/BLUEPRINTS/Interactables/DestructableMesh/DRONE_FS_MasterField.FieldLifespan` 0.1 (`self.DestructionREF`))
        (set `/Game/BLUEPRINTS/Interactables/DestructableMesh/DRONE_FS_MasterField.Radial Magnitude` 150.0 (`self.DestructionREF`))
        (`/Game/BLUEPRINTS/Interactables/DestructableMesh/DRONE_FS_MasterField.CE_Trigger` (`self.DestructionREF`))
        (`KismetSystemLibrary.Delay` 0.3)))))

(event `self.ReceiveBeginPlay`
  (`|ExecutionSequence`
    (:`then_0`
      (bind _asai_drone_controller (cast `/Game/BLUEPRINTS/DRONE_AI/AI_DroneLogic/AI_DroneController` (`self.GetController`)))
      (set `self.DroneREF` _asai_drone_controller)
      (set `self.CurrentHealth` (`self.MaxHealth`))
      (bind _asai_drone_healthbar (cast `/Game/BLUEPRINTS/UI/AI_DroneHealthbar` (`WidgetComponent.GetUserWidgetObject` (`self.HealthBar`))))
      (set `/Game/BLUEPRINTS/UI/AI_DroneHealthbar.Owner` self _asai_drone_healthbar))
    (:`then_1`
      ;[1 1 1] Movement Tick
      (`self.CheckCanPatrol`)
      (bind _returnvalue (`KismetSystemLibrary.K2_SetTimerDelegate` (delegate `MovementTickRate`) (`self.MovementTime`) true))
      (set `self.MovementTimer` _returnvalue)
      ;[1 1 1] PlayerMovementTick
      (bind _returnvalue_2 (`KismetSystemLibrary.K2_SetTimerDelegate` (delegate `PlayerTickRate`) (`self.PlayerTime`) true))
      (set `self.CheckForPlayer` _returnvalue_2)
      ;[1 1 1] Drone Shoot Tick rate
      (bind _returnvalue_3 (`KismetSystemLibrary.K2_SetTimerDelegate` (delegate `ShootTick`) (`self.ShootTickRate`) true))
      (set `self.ShootTimer` _returnvalue_3))))

(event `Patrol`
  (bind _output (`|GetArrayItem` (`self.PatrolPoints`) (`self.PatrolIndex`)))
  ;[1 1 1] Patrol
  (if (`self.CanPatrol`)
    (if (< (`self.GetDistanceTo` self _output) (`self.AcceptanceRadius`))
      (`self.NextPatrolLocation`)
      (else
        (`self.GoTo` true true (`self.K2_GetActorLocation` _output))))))

(event `PlayerTickRate`
  ;[1 1 1] PlayerMovementTick
  (bind (_targetfound _location) (`self.TracePlayer`))
  (if _targetfound
    (set `self.LastPlayerLocation` _location)
    (set `self.FlyModes` "NewEnumerator1")
    (else
      (switch `/Game/BLUEPRINTS/DRONE_AI/AI_DroneLogic/E_FlyModes` (`self.FlyModes`)
        (:`NewEnumerator1`
          (set `self.FlyModes` "NewEnumerator2")
          (set `self.PlayerCounter` 0))))))

(event `ShootTick`
  ;[1 1 1] Drone Shoot Tick rate
  (`self.CanShoot?`))

(event `MovementTickRate`
  ;[1 1 1] Movement Tick
  (switch `/Game/BLUEPRINTS/DRONE_AI/AI_DroneLogic/E_FlyModes` (`self.FlyModes`)
    (:`NewEnumerator0`
      (`self.Patrol`))
    (:`NewEnumerator1`
      (`self.Aggro`))
    (:`NewEnumerator2`
      (`self.LookingForPlayer`))))

(event `GoTo`
  (params (ForwardMovement :type Boolean) (Rotation :type Boolean) (Location :type "Vector Structure"))
  (bind _aggroinginterpolationspeed (`self.AggroingInterpolationSpeed`))
  (bind _aggroing (`self.Aggroing`))
  ;[1 1 1] Drone movement
  (`|ExecutionSequence`
    (:`then_0`
      (if ForwardMovement
        (`PawnMovementComponent.AddInputVector` (`self.FloatingPawnMovement`) (* (`self.GetActorForwardVector`) (select `/Game/BLUEPRINTS/DRONE_AI/AI_DroneLogic/E_FlyModes` (`self.FlyModes`) :`NewEnumerator0` (`self.Patrolling`) :`NewEnumerator1` _aggroing :`NewEnumerator2` _aggroing)) false)))
    (:`then_1`
      (if Rotation
        (`self.K2_SetActorRotation` (`KismetMathLibrary.RInterpTo` (`self.K2_GetActorRotation`) (`KismetMathLibrary.Conv_VectorToRotator` (`KismetMathLibrary.Normal` (- Location (`self.K2_GetActorLocation`)))) (`self.MovementTime`) (select `/Game/BLUEPRINTS/DRONE_AI/AI_DroneLogic/E_FlyModes` (`self.FlyModes`) :`NewEnumerator0` (`self.PatrollingInerpolationSpeed`) :`NewEnumerator1` _aggroinginterpolationspeed :`NewEnumerator2` _aggroinginterpolationspeed)))))))

(event `/Game/BLUEPRINTS/TakeDamage.ITakeDamage`
  (params (BoneName :type Name) (Damage :type "Float (double-precision)"))
  (bind _returnvalue (`self.K2_GetActorLocation`))
  (bind _base (`self.Base`))
  (if (== BoneName "Head")
    (set `self.CurrentHealth` 0.0)
    (else
      (bind _output_get (set `self.CurrentHealth` (- (`self.CurrentHealth`) Damage)))))
  (if (<= _output_get 0.0)
    (set `self.Dead?` true)
    (set `self.CanPatrol` false)
    (`GameplayStatics.SpawnSoundAtLocation` "/Game/BLUEPRINTS/Sounds/Interaction/Electronics_Cue.Electronics_Cue" _returnvalue (struct) 1.0 1.0 0.0 null null)
    (`GameplayStatics.SpawnEmitterAttached` "/Game/BLUEPRINTS/DRONE_AI/AI_DroneLogic/SW_Drone/Particles/P_Explosion.P_Explosion" (`self.Base`) "None" _returnvalue (`self.K2_GetActorRotation`) (3.0 3.0 3.0) "KeepWorldPosition")
    (`GameplayStatics.PlaySoundAtLocation` "/Game/BLUEPRINTS/ITEM_Pickups/Weapons/SciFiWeapLight/Sound/GrenadeLauncher/GL_Explosion_Cue.GL_Explosion_Cue" _returnvalue (struct) 1.0 1.0 0.0 null null null null)
    (`KismetSystemLibrary.Delay` 0.2)
    (`SceneComponent.SetHiddenInGame` (`self.Base`) true true)
    (`|SpawnActorFromClass` "/Game/BLUEPRINTS/DRONE_AI/AI_DroneLogic/BlownUpDroneBP.BlownUpDroneBP_C" (`KismetMathLibrary.MakeTransform` (`SceneComponent.K2_GetComponentLocation` _base) (`SceneComponent.K2_GetComponentRotation` _base)) "Undefined" "OverrideRootScale" null null)
    (if (`self.Dead?`)
      (bind _asdevatox_bp (cast `/Game/BLUEPRINTS/DevatoxBP` (`GameplayStatics.GetPlayerCharacter` 0)))
      (`/Game/BLUEPRINTS/UI/PlayerHUD.UpdateTargets` (`/Game/BLUEPRINTS/DevatoxBP.PlayerHUDref` _asdevatox_bp) (`self.Enemy Killed`))
      (`self.K2_DestroyActor`))))

(event `Aggro`
  ;[1 1 1] Player character trace last known location and Aggro
  (if (> (`KismetMathLibrary.VSize` (- (`self.K2_GetActorLocation`) (`self.LastPlayerLocation`))) (`self.AggroAcceptanceRadius`))
    (`self.GoTo` true true (`self.LastPlayerLocation`))
    (else
      (`self.GoTo` false true (`self.LastPlayerLocation`))
      (set `MovementComponent.Velocity` (0.0 0.0 0.0) (`self.FloatingPawnMovement`)))))

(event `LookingForPlayer`
  ;[1 1 1] Player character trace last known location and Aggro
  (if (> (`KismetMathLibrary.VSize` (- (`self.K2_GetActorLocation`) (`self.LastPlayerLocation`))) (`self.AggroAcceptanceRadius`))
    (`self.GoTo` true true (`self.LastPlayerLocation`))
    (else
      (set `MovementComponent.Velocity` (0.0 0.0 0.0) (`self.FloatingPawnMovement`))
      (bind _result (`/Engine/EditorBlueprintResources/StandardMacros.IncrementInt` (`self.PlayerCounter`))
        (:`  `
          (if (> _result (`self.MaxPlayer`))
            (set `self.FlyModes` "NewEnumerator0")
            (else
              (`self.K2_AddActorWorldRotation` (`KismetMathLibrary.MakeRotator` 0.0 0.0 (/ (`self.MaxPlayer`) 360))))))))))

(fn `CheckCanPatrol`
  (if (> (`KismetArrayLibrary.Array_Length` (`self.PatrolPoints`)) 0)
    (for _array_element (`self.PatrolPoints`)
      (`/Engine/EditorBlueprintResources/StandardMacros.IsValid` _array_element
        (:`Is Not Valid`
          (`/Engine/EditorBlueprintResources/StandardMacros.IncrementInt` (`self.InvalidIndexs`)))))
    (set `self.CanPatrol` (not (== (`self.InvalidIndexs`) (`KismetArrayLibrary.Array_Length` (`self.PatrolPoints`)))))
    (else
      (set `self.CanPatrol` false))))

(fn `NextPatrolLocation`
  (bind _returnvalue (+ (`self.PatrolIndex`) 1))
  (bind _output_get (set `self.PatrolIndex` (`KismetMathLibrary.SelectInt` 0 _returnvalue (== _returnvalue (`KismetArrayLibrary.Array_Length` (`self.PatrolPoints`)))) :!label _label))
  (`/Engine/EditorBlueprintResources/StandardMacros.IsValid` (`|GetArrayItem` (`self.PatrolPoints`) _output_get)
    (:`Is Not Valid`
      (goto _label))))

(fn `TracePlayer`
  (returns (TargetFound :type Boolean) (Location :type "Vector Structure"))
  (bind _returnvalue (`SceneComponent.K2_GetComponentLocation` (`self.FowardVector`)))
  (bind _returnvalue_2 (`KismetMathLibrary.Normal` (- (`self.K2_GetActorLocation` (`GameplayStatics.GetPlayerCharacter` 0)) (`self.K2_GetActorLocation`))))
  (if (> (`KismetMathLibrary.Dot_VectorVector` (`SceneComponent.GetForwardVector` (`self.FowardVector`)) _returnvalue_2) (`self.FindPlayerDOT`))
    (bind (_outhit _returnvalue_3) (`KismetSystemLibrary.LineTraceSingleForObjects` _returnvalue (+ _returnvalue (* _returnvalue_2 (`self.TraceDistance`))) (`|MakeArray` "ObjectTypeQuery1" "ObjectTypeQuery2" "ObjectTypeQuery3" "ObjectTypeQuery4" "ObjectTypeQuery6" :!type "EObjectTypeQuery Enum")))
    (if _returnvalue_3
      (bind (_bblockinghit _binitialoverlap _time _distance _location _impactpoint _normal _impactnormal _physmat _hitactor) (`GameplayStatics.BreakHitResult` _outhit))
      (return (== (`GameplayStatics.GetPlayerCharacter` 0) _hitactor) _impactpoint)
      (else
        (return false (0.0 0.0 0.0))))))

(fn `UserConstructionScript`
  (bind (_droninfo_dronetype _droninfo_class _droninfo_maxhealth _droninfo_damage _droninfo_range _droninfo_attackdistance _droninfo_projectile _droninfo_dronefiresound) (break `/Game/BLUEPRINTS/DRONE_AI/AI_DroneLogic/DroneInfo` (`self.DronInfo`)))
  (set `self.DronInfo` (make `/Game/BLUEPRINTS/DRONE_AI/AI_DroneLogic/DroneInfo` _droninfo_dronetype (`GameplayStatics.GetObjectClass` self) _droninfo_maxhealth _droninfo_damage _droninfo_range _droninfo_attackdistance _droninfo_projectile _droninfo_dronefiresound)))