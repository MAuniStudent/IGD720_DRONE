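; Automated twin-gun turret that picks visible pawns in range, turns toward them and shoots.
; Tick runs target search, clamped-pitch rotation and firing, gated by fire rate and a dot-product aim check.
; Each gun line-traces, then spawns a projectile, effects and a short-lived Chaos field at impact, and plays a recoil timeline.
; Gun one damages the hit actor through the TakeDamage interface, while gun two targets the player character.
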(event `self.ReceiveBeginPlay`
  (`TimelineComponent.SetFloatCurve` (`self.GunOneRecoil`) "/Game/BLUEPRINTS/DRONE_AI/Turrets/Recoil.Recoil" "recoilL")
  (`TimelineComponent.SetFloatCurve` (`self.GunTwoRecoil`) "/Game/BLUEPRINTS/DRONE_AI/Turrets/Recoil.Recoil" "recoilR"))

(event `self.ReceiveTick`
  (params (DeltaSeconds :type "Float (single-precision)"))
  (`self.FindBestTarget`)
  (`self.TurretTarget`
    (:`then`
      (`self.UpdateRotation` DeltaSeconds)
      (`self.TurretFire`))
    (:`else`)))

(event `Fire`
  (bind _projectileone (`self.ProjectileONe`))
  (bind _projectileone_2 (`self.ProjectileONe`))
  (bind _projectiletwo (`self.ProjectileTwo`))
  (bind _projectiletwo_2 (`self.ProjectileTwo`))
  (bind _returnvalue (`SceneComponent.K2_GetComponentLocation` _projectileone))
  (bind _returnvalue_2 (`SceneComponent.K2_GetComponentLocation` (`self.ProjectileONe`)))
  (bind _returnvalue_3 (`SceneComponent.K2_GetComponentLocation` _projectiletwo))
  (bind _returnvalue_4 (`SceneComponent.K2_GetComponentLocation` (`self.ProjectileTwo`)))
  (bind (_asdevatox_bp _bsuccess) (cast `/Game/BLUEPRINTS/DevatoxBP` (`GameplayStatics.GetPlayerCharacter` 0) :!pure true))
  (set `self.LastFire` (`KismetSystemLibrary.GetGameTimeInSeconds`))
  (`|ExecutionSequence`
    (:`then_0`
      (goto _label :!via `Reset`))
    (:`then_1`
      (`/Engine/EditorBlueprintResources/StandardMacros.Do N` 2 :!label _label
        (:`Exit`
          (bind _outactors (`GameplayStatics.GetAllActorsWithTag` "NoTurretFire"))
          (bind (_outhit _returnvalue_5) (`KismetSystemLibrary.LineTraceSingle` _returnvalue (+ _returnvalue (* (`SceneComponent.GetForwardVector` _projectileone) (`self.TurretRange`))) "TraceTypeQuery1" false _outactors))
          (if _returnvalue_5
            _
            (else
              _))
          (`GameplayStatics.PlaySound2D` "/Game/BLUEPRINTS/Sounds/Interaction/gun_heavy_Cue.gun_heavy_Cue" 0.25 0.7 0.0 null null)
          (bind (_bblockinghit _binitialoverlap _time _distance _location _impactpoint _normal _impactnormal _physmat _hitactor _hitcomponent _hitbonename _bonename _hititem _elementindex _faceindex _tracestart _traceend) (`GameplayStatics.BreakHitResult` _outhit))
          (if (`KismetSystemLibrary.DoesImplementInterface` _hitactor "/Game/BLUEPRINTS/TakeDamage.TakeDamage_C")
            (message `/Game/BLUEPRINTS/TakeDamage.ITakeDamage` _hitactor _hitbonename 50.0))
          (bind (_returnvalue_location _returnvalue_rotation) (`KismetMathLibrary.BreakTransform` (`KismetMathLibrary.MakeTransform` _returnvalue_2 (`KismetMathLibrary.FindLookAtRotation` _returnvalue_2 (`KismetMathLibrary.SelectVector` _impactpoint _traceend _returnvalue_5)))))
          (bind _returnvalue_6 (`|SpawnActorFromClass` "/Game/BLUEPRINTS/DRONE_AI/Turrets/TurretProjectile.TurretProjectile_C" (`KismetMathLibrary.MakeTransform` _returnvalue_location _returnvalue_rotation) "Undefined" "MultiplyWithRoot" null null))
          (`TimelineComponent.PlayFromStart` (`self.GunOneRecoil`))
          (`NiagaraFunctionLibrary.SpawnSystemAtLocation` "/Game/BLUEPRINTS/FX/sA_Megapack_v1/sA_Projectilevfx/Vfx/Fx/Niagara_Systems/NS_Hit5.NS_Hit5" _impactnormal)
          (`PrimitiveComponent.AddImpulseAtLocation` (`/Game/BLUEPRINTS/ITEM_Pickups/Weapons/ProjectileBaseBP.Sphere` _returnvalue_6) (* (`self.GetVelocity`) 100.0) (`self.K2_GetActorLocation`) "None")
          (`GameplayStatics.SpawnEmitterAttached` "/Game/BLUEPRINTS/ITEM_Pickups/Weapons/SciFiWeapLight/FX/Particles/P_AssaultRifle_MuzzleFlash_Dark.P_AssaultRifle_MuzzleFlash_Dark" _projectileone_2 "None" (`SceneComponent.K2_GetComponentLocation` _projectileone_2) (`SceneComponent.K2_GetComponentRotation` _projectileone_2) (1.0 1.0 1.0) "KeepWorldPosition")
          (bind (_returnvalue_location_2 _returnvalue_rotation_2) (`KismetMathLibrary.BreakTransform` (`KismetMathLibrary.Conv_VectorToTransform` _impactpoint)))
          (bind _returnvalue_7 (`|SpawnActorFromClass` "/Game/BLUEPRINTS/Interactables/DestructableMesh/DRONE_FS_MasterField.DRONE_FS_MasterField_C" (`KismetMathLibrary.MakeTransform` (+ _returnvalue_location_2 (* _impactnormal (-3.0 -3.0 -3.0))) _returnvalue_rotation_2) "Undefined" "MultiplyWithRoot" null null))
          (set `self.ChaosBoomREF` _returnvalue_7)
          (set `/Game/BLUEPRINTS/Interactables/DestructableMesh/DRONE_FS_MasterField.ActivationType` "NewEnumerator4" (`self.ChaosBoomREF`))
          (set `/Game/BLUEPRINTS/Interactables/DestructableMesh/DRONE_FS_MasterField.FieldLifespan` 0.1 (`self.ChaosBoomREF`))
          (set `/Game/BLUEPRINTS/Interactables/DestructableMesh/DRONE_FS_MasterField.Radial Magnitude` 150.0 (`self.ChaosBoomREF`))
          (`/Game/BLUEPRINTS/Interactables/DestructableMesh/DRONE_FS_MasterField.CE_Trigger` (`self.ChaosBoomREF`))
          (`KismetSystemLibrary.Delay` 0.5)
          (bind _outactors_2 (`GameplayStatics.GetAllActorsOfClassWithTag` "/Game/BLUEPRINTS/DRONE_AI/AI_InfantryLogic/AI_BaseWalking.AI_BaseWalking_C" "NoTurretFire"))
          (bind (_outhit_2 _returnvalue_8) (`KismetSystemLibrary.LineTraceSingle` _returnvalue_3 (+ _returnvalue_3 (* (`SceneComponent.GetForwardVector` _projectiletwo) (`self.TurretRange`))) "TraceTypeQuery1" true _outactors_2))
          (if _returnvalue_8
            _
            (else
              _))
          (`GameplayStatics.PlaySound2D` "/Game/BLUEPRINTS/Sounds/Interaction/gun_heavy_Cue.gun_heavy_Cue" 0.25 1.0 0.0 null null)
          (bind (_bblockinghit_2 _binitialoverlap_2 _time_2 _distance_2 _location_2 _impactpoint_2 _normal_2 _impactnormal_2 _physmat_2 _hitactor_2 _hitcomponent_2 _hitbonename_2 _bonename_2 _hititem_2 _elementindex_2 _faceindex_2 _tracestart_2 _traceend_2) (`GameplayStatics.BreakHitResult` _outhit_2))
          (if (== (`KismetSystemLibrary.DoesImplementInterface` _hitactor_2 "/Game/BLUEPRINTS/TakeDamage.TakeDamage_C") _bsuccess)
            (message `/Game/BLUEPRINTS/TakeDamage.ITakeDamage` _asdevatox_bp _hitbonename_2 50.0))
          (bind (_returnvalue_location_3 _returnvalue_rotation_3) (`KismetMathLibrary.BreakTransform` (`KismetMathLibrary.MakeTransform` _returnvalue_4 (`KismetMathLibrary.FindLookAtRotation` _returnvalue_4 (`KismetMathLibrary.SelectVector` _impactpoint_2 _traceend_2 _returnvalue_8)))))
          (bind _returnvalue_9 (`|SpawnActorFromClass` "/Game/BLUEPRINTS/DRONE_AI/Turrets/TurretProjectile.TurretProjectile_C" (`KismetMathLibrary.MakeTransform` _returnvalue_location_3 _returnvalue_rotation_3 (2.0 2.0 2.0)) "Undefined" "MultiplyWithRoot" null null))
          (`TimelineComponent.PlayFromStart` (`self.GunTwoRecoil`))
          (`NiagaraFunctionLibrary.SpawnSystemAtLocation` "/Game/BLUEPRINTS/FX/sA_Megapack_v1/sA_Projectilevfx/Vfx/Fx/Niagara_Systems/NS_Hit5.NS_Hit5" _location_2)
          (`PrimitiveComponent.AddImpulseAtLocation` (`/Game/BLUEPRINTS/ITEM_Pickups/Weapons/ProjectileBaseBP.Sphere` _returnvalue_9) (* (`self.GetVelocity`) 100.0) (`self.K2_GetActorLocation`) "None")
          (`GameplayStatics.SpawnEmitterAttached` "/Game/BLUEPRINTS/ITEM_Pickups/Weapons/SciFiWeapLight/FX/Particles/P_AssaultRifle_MuzzleFlash_Dark.P_AssaultRifle_MuzzleFlash_Dark" _projectiletwo_2 "None" (`SceneComponent.K2_GetComponentLocation` _projectiletwo_2) (`SceneComponent.K2_GetComponentRotation` _projectiletwo_2) (1.0 1.0 1.0) "KeepWorldPosition")
          (bind (_returnvalue_location_4 _returnvalue_rotation_4) (`KismetMathLibrary.BreakTransform` (`KismetMathLibrary.Conv_VectorToTransform` _impactpoint_2)))
          (bind _returnvalue_10 (`|SpawnActorFromClass` "/Game/BLUEPRINTS/Interactables/DestructableMesh/DRONE_FS_MasterField.DRONE_FS_MasterField_C" (`KismetMathLibrary.MakeTransform` (+ _returnvalue_location_4 (* _impactnormal_2 (-3.0 -3.0 -3.0))) _returnvalue_rotation_4) "Undefined" "MultiplyWithRoot" null null))
          (set `self.ChaosBoomREF` _returnvalue_10)
          (set `/Game/BLUEPRINTS/Interactables/DestructableMesh/DRONE_FS_MasterField.ActivationType` "NewEnumerator4" (`self.ChaosBoomREF`))
          (set `/Game/BLUEPRINTS/Interactables/DestructableMesh/DRONE_FS_MasterField.FieldLifespan` 0.1 (`self.ChaosBoomREF`))
          (set `/Game/BLUEPRINTS/Interactables/DestructableMesh/DRONE_FS_MasterField.Radial Magnitude` 150.0 (`self.ChaosBoomREF`))
          (`/Game/BLUEPRINTS/Interactables/DestructableMesh/DRONE_FS_MasterField.CE_Trigger` (`self.ChaosBoomREF`))
          (`KismetSystemLibrary.Delay` 0.3)
          (goto _label))))))

(fn `FindBestTarget`
  (locals (Best :type "Float (double-precision)") (BestTarget :type "Actor Object Reference") (CurrentTarget :type "Actor Object Reference") (Current :type "Float (double-precision)"))
  (set `local.Best` (+ (`self.TurretRange`) 1.0))
  (bind _outactors (`KismetSystemLibrary.SphereOverlapActors` (`self.K2_GetActorLocation`) (`self.TurretRange`) (`|MakeArray` "ObjectTypeQuery3" :!type "EObjectTypeQuery Enum") "/Script/Engine.Actor"))
  (for _array_element _outactors
    (bind _output_get (set `local.CurrentTarget` _array_element))
    (bind _output_get_2 (set `local.Current` (`self.GetDistanceTo` _output_get self)))
    (if (or (< _output_get_2 (`local.Best`)) (`KismetSystemLibrary.IsValid` (`local.BestTarget`)))
      (bind _targetresult (`/Game/BLUEPRINTS/MyFunction.HasLineOfSight` (`SceneComponent.K2_GetComponentLocation` (`self.Turret`)) (`self.K2_GetActorLocation` (`local.CurrentTarget`)) (`|MakeArray` self (`local.CurrentTarget`) :!type "Actor Object Reference")))
      (if _targetresult
        (set `local.BestTarget` (`local.CurrentTarget`))
        (set `local.Best` (`local.Current`)))))
  (set `self.TurretTarget` (`local.BestTarget`)))

(fn `TurretFire`
  (if (> (- (`KismetSystemLibrary.GetGameTimeInSeconds`) (`self.LastFire`)) (`self.FireRate`))
    (if (> (`KismetMathLibrary.Dot_VectorVector` (`KismetMathLibrary.GetDirectionUnitVector` (`SceneComponent.K2_GetComponentLocation` (`self.TurretBase`)) (`self.K2_GetActorLocation` (`self.TurretTarget`))) (`SceneComponent.GetForwardVector` (`self.Turret`))) 0.99)
      (`self.Fire`))))

(fn `UpdateRotation`
  (params (Delta :type "Float (double-precision)"))
  (bind _output_get (set `self.TargetRotation` (`KismetMathLibrary.RInterpTo_Constant` (`SceneComponent.K2_GetComponentRotation` (`self.Turret`)) (`KismetMathLibrary.FindLookAtRotation` (`SceneComponent.K2_GetComponentLocation` (`self.Turret`)) (`self.K2_GetActorLocation` (`self.TurretTarget`))) (`local.Delta`) (`self.Interp Speed`))))
  (`SceneComponent.K2_SetWorldRotation` (`self.Turret`) (`KismetMathLibrary.MakeRotator` (.roll _output_get) (`KismetMathLibrary.ClampAngle` (.pitch _output_get) -45.0 75.0) (.yaw _output_get)) false false))

(fn `UserConstructionScript`)