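; AI controller for AI_BaseWalking enemies that patrols waypoints and attacks the player.
; Patrol chains waypoint moves with pauses until a looping CheckStatus timer reads the pawn's enemy-found flag and starts Hunting.
; CheckStatus also resumes patrol when the player dies and stops when the pawn dies.
; Weapon fire applies random damage by line trace through the TakeDamage interface, plus a projectile, sound and effects.
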(event `self.ReceiveBeginPlay`
  (bind _asai_base_walking (cast `/Game/BLUEPRINTS/DRONE_AI/AI_BaseWalking` (`self.K2_GetPawn`)))
  (bind _output_get (set `self.As AI Base Walking` _asai_base_walking))
  (set `self.Waypoints` (`/Game/BLUEPRINTS/DRONE_AI/AI_BaseWalking.Waypoint` _output_get))
  (bind _returnvalue (`KismetSystemLibrary.K2_SetTimer` null "CheckStatus" 0.3 true))
  (set `self.JobDone` _returnvalue)
  (`|AIMoveTo` (`self.As AI Base Walking`) (0.0 0.0 0.0) (`|GetArrayItem` (`self.Waypoints`) (`self.CurrentPosition`))
    (:`OnSuccess`
      (`KismetSystemLibrary.Delay` 3.0)
      (`self.Patrol`))))

(event `Patrol`
  (if (not (`self.FoundEnemy`))
    (if (`self.TurnAround`)
      (`/Engine/EditorBlueprintResources/StandardMacros.DecrementInt` (`self.CurrentPosition`)
        (:`  `
          (`|AIMoveTo` (`self.As AI Base Walking`) (0.0 0.0 0.0) (`|GetArrayItem` (`self.Waypoints`) (`self.CurrentPosition`))
            (:`OnSuccess`
              (if (<= (`self.CurrentPosition`) 0)
                (set `self.TurnAround` false))))))
      (else
        (`/Engine/EditorBlueprintResources/StandardMacros.DecrementInt` (`self.CurrentPosition`)
          (:`  `
            (`|AIMoveTo` (`self.As AI Base Walking`) (0.0 0.0 0.0) (`|GetArrayItem` (`self.Waypoints`) (`self.CurrentPosition`))
              (:`OnSuccess`
                (if (>= (`self.CurrentPosition`) (- (`KismetArrayLibrary.Array_Length` (`self.Waypoints`)) 1))
                  (set `self.TurnAround` true))))))))
    (`KismetSystemLibrary.Delay` (`KismetMathLibrary.RandomFloatInRange` 2.0 5.0))
    (`self.Patrol`)))

(event `Hunting`
  (`|AIMoveTo` (`self.As AI Base Walking`) (0.0 0.0 0.0) (`GameplayStatics.GetPlayerCharacter` 0) 1000.0
    (:`OnSuccess`
      (`self.AI_FireWeapon`))))

(event `CheckStatus`
  (bind _as_ai_base_walking (`self.As AI Base Walking`))
  (if (`/Game/BLUEPRINTS/DevatoxBP.IsDead?` (cast `/Game/BLUEPRINTS/DevatoxBP` (`GameplayStatics.GetPlayerCharacter` 0) :!pure true))
    (set `self.FoundEnemy` false)
    (`/Engine/EditorBlueprintResources/StandardMacros.DoOnce` false
      (:`Completed`
        (`/Game/BLUEPRINTS/DRONE_AI/AI_BaseWalking.ExitCombat` (`self.As AI Base Walking`))
        (`GameplayStatics.PlaySound2D` "/Game/BLUEPRINTS/Sounds/Interaction/target-destroyed_Cue.target-destroyed_Cue" 1.0 1.0 0.0 null null)
        (`self.Patrol`)))
    (elif (`/Game/BLUEPRINTS/DRONE_AI/AI_BaseWalking.IsDead?` _as_ai_base_walking)
      (`KismetSystemLibrary.K2_ClearAndInvalidateTimerHandle` (`self.JobDone`))
      (`self.StopMovement`)
      (else
        (bind _output_get (set `self.FoundEnemy` (`/Game/BLUEPRINTS/DRONE_AI/AI_BaseWalking.EnemeyFound` _as_ai_base_walking)))
        (if _output_get
          (`|ExecutionSequence`
            (:`then_0`
              (`self.Hunting`))
            (:`then_1`
              (`/Engine/EditorBlueprintResources/StandardMacros.DoOnce` false
                (:`Completed`
                  (`/Game/BLUEPRINTS/DRONE_AI/AI_BaseWalking.EnableCombat` (`self.As AI Base Walking`)))))))))))

(event `AI_FireWeapon`
  (bind _aiweaponref (`/Game/BLUEPRINTS/DRONE_AI/AI_BaseWalking.AIWeaponREF` (`self.As AI Base Walking`)))
  (bind _projectilespawnpoint (`/Game/BLUEPRINTS/ITEM_Pickups/Weapons/masterWeaponBP.ProjectileSpawnPoint` (`/Game/BLUEPRINTS/DRONE_AI/AI_BaseWalking.AIWeaponREF` (`self.As AI Base Walking`))))
  (bind _projectilespawnpoint_2 (`/Game/BLUEPRINTS/ITEM_Pickups/Weapons/masterWeaponBP.ProjectileSpawnPoint` (`/Game/BLUEPRINTS/DRONE_AI/AI_BaseWalking.AIWeaponREF` (`self.As AI Base Walking`))))
  (bind _returnvalue (`SceneComponent.K2_GetComponentLocation` _projectilespawnpoint_2))
  (bind _returnvalue_2 (`SceneComponent.K2_GetComponentLocation` (`/Game/BLUEPRINTS/ITEM_Pickups/Weapons/masterWeaponBP.ProjectileSpawnPoint` _aiweaponref)))
  (bind (_outhit _returnvalue_3) (`KismetSystemLibrary.LineTraceSingle` _returnvalue (+ _returnvalue (* (`SceneComponent.GetForwardVector` _projectilespawnpoint_2) 15000.0)) "TraceTypeQuery1" true))
  (if _returnvalue_3
    _
    (else
      _))
  (`GameplayStatics.PlaySound2D` (`.Sound_55_F227351C473F0825862A5E9026DEF617` (break `/Game/BLUEPRINTS/ITEM_Pickups/Weapons/WeaponInfo` (`/Game/BLUEPRINTS/ITEM_Pickups/Weapons/masterWeaponBP.WeaponInfo` _aiweaponref))) 1.0 1.0 0.0 null null)
  (bind (_bblockinghit _binitialoverlap _time _distance _location _impactpoint _normal _impactnormal _physmat _hitactor _hitcomponent _hitbonename _bonename _hititem _elementindex _faceindex _tracestart _traceend) (`GameplayStatics.BreakHitResult` _outhit))
  (if (`KismetSystemLibrary.DoesImplementInterface` _hitactor "/Game/BLUEPRINTS/TakeDamage.TakeDamage_C")
    (message `/Game/BLUEPRINTS/TakeDamage.ITakeDamage` _hitactor _hitbonename (`KismetMathLibrary.RandomFloatInRange` 20.0 35.0)))
  (bind (_returnvalue_location _returnvalue_rotation) (`KismetMathLibrary.BreakTransform` (`KismetMathLibrary.MakeTransform` _returnvalue_2 (`KismetMathLibrary.FindLookAtRotation` _returnvalue_2 (`KismetMathLibrary.SelectVector` _impactpoint _traceend _returnvalue_3)))))
  (`|SpawnActorFromClass` "/Game/BLUEPRINTS/ITEM_Pickups/Weapons/AI_Projectiles/AI_AssaultRifleProjectile.AI_AssaultRifleProjectile_C" (`KismetMathLibrary.MakeTransform` _returnvalue_location _returnvalue_rotation) "Undefined" "MultiplyWithRoot" null null)
  (`GameplayStatics.SpawnEmitterAtLocation` "/Game/BLUEPRINTS/ITEM_Pickups/Weapons/SciFiWeapLight/FX/Particles/P_Impact_Metal_Large_Dark.P_Impact_Metal_Large_Dark" _location)
  (`GameplayStatics.SpawnEmitterAttached` "/Game/BLUEPRINTS/ITEM_Pickups/Weapons/SciFiWeapLight/FX/Particles/P_AssaultRifle_MuzzleFlash_Dark.P_AssaultRifle_MuzzleFlash_Dark" _projectilespawnpoint "None" (`SceneComponent.K2_GetComponentLocation` _projectilespawnpoint) (`SceneComponent.K2_GetComponentRotation` _projectilespawnpoint) (1.0 1.0 1.0) "KeepWorldPosition"))

(fn `UserConstructionScript`)