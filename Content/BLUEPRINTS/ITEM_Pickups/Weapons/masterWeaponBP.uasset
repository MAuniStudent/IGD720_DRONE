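; Master weapon pickup Blueprint that shows an info widget and lets the DevatoxBP character pick it up.
; Sphere overlap toggles the widget and pickup flag, fills in name and icon, and enables input so IA_Interaction calls the character's WeaponPickup.
; A looping timer turns the widget toward the camera, and cleanup events remove the sphere or hide the prompt.
; The construction script writes the actor's own class into its WeaponInfo struct.
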(event `StartTimer`
  (`KismetSystemLibrary.K2_SetTimerDelegate` (delegate `WidgetRotation`) 0.2 true))

(event `WidgetRotation`
  (bind _widget (`self.Widget`))
  (`SceneComponent.K2_SetWorldRotation` _widget (`KismetMathLibrary.FindLookAtRotation` (`SceneComponent.K2_GetComponentLocation` _widget) (`PlayerCameraManager.GetCameraLocation` (`GameplayStatics.GetPlayerCameraManager` 0))) false false))

(event `self.ReceiveBeginPlay`
  (`self.StartTimer`))

(event `self.Sphere.OnComponentBeginOverlap`
  (params (OverlappedComponent :type "PrimitiveComponent Object Reference") (OtherActor :type "Actor Object Reference") (OtherComp :type "PrimitiveComponent Object Reference") (OtherBodyIndex :type Integer) (bFromSweep :type Boolean) (SweepResult :type "HitResult Structure (by ref)"))
  (bind ((`Name_9_1090D52F4EF75D15339E1AB0A367F2A4` _name) (`Image_12_8EE979984178E8A6911405B743FDA336` _image)) (break `/Game/BLUEPRINTS/ITEM_Pickups/Weapons/WeaponInfo` (`self.WeaponInfo`)))
  (bind _asweapon_pickup_wb (cast `/Game/BLUEPRINTS/UI/WeaponPickupWB` (`WidgetComponent.GetUserWidgetObject` (`self.Widget`)) :!pure true))
  (bind _asdevatox_bp (cast `/Game/BLUEPRINTS/DevatoxBP` OtherActor))
  (set `self.As Devatox BP` _asdevatox_bp)
  (`SceneComponent.SetVisibility` (`self.Widget`) true false)
  (set `self.CanPickup?` true)
  (`self.EnableInput` (`GameplayStatics.GetPlayerController` 0))
  (set `/Game/BLUEPRINTS/UI/WeaponPickupWB.WeaponInfo` (`KismetTextLibrary.Conv_StringToText` _name) _asweapon_pickup_wb)
  (set `/Game/BLUEPRINTS/UI/WeaponPickupWB.WeaponIcon` _image _asweapon_pickup_wb))

(event `self.Sphere.OnComponentEndOverlap`
  (params (OverlappedComponent :type "PrimitiveComponent Object Reference") (OtherActor :type "Actor Object Reference") (OtherComp :type "PrimitiveComponent Object Reference") (OtherBodyIndex :type Integer))
  (bind _asdevatox_bp (cast `/Game/BLUEPRINTS/DevatoxBP` OtherActor))
  (set `self.As Devatox BP` _asdevatox_bp)
  (`SceneComponent.SetVisibility` (`self.Widget`) false false)
  (set `self.CanPickup?` false))

(event `EnhancedInput|/Game/BLUEPRINTS/Input/Actions/IA_Interaction`
  (params (ActionValue :type Boolean) (ElapsedSeconds :type "Float (double-precision)") (TriggeredSeconds :type "Float (double-precision)") (InputAction :type "InputAction Object Reference" :default "/Game/BLUEPRINTS/Input/Actions/IA_Interaction.IA_Interaction"))
  (:`Started`
    (if (`self.CanPickup?`)
      (`/Game/BLUEPRINTS/DevatoxBP.WeaponPickup` (`self.As Devatox BP`) self))))

(event `CleanShit`
  (`ActorComponent.K2_DestroyComponent` (`self.Sphere`))
  (`SceneComponent.SetVisibility` (`self.Widget`) false false)
  (set `self.CanPickup?` false))

(event `DestroySphere`
  (`ActorComponent.K2_DestroyComponent` (`self.Sphere`)))

(fn `UserConstructionScript`
  (bind (_weaponinfo_weapontype _weaponinfo_classs _weaponinfo_name _weaponinfo_image _weaponinfo_equipsocket _weaponinfo_unequipsocket _weaponinfo_firerate _weaponinfo_damage _weaponinfo_range _weaponinfo_sound _weaponinfo_ammotype _weaponinfo_clipsize _weaponinfo_currentammo _weaponinfo_maxammo _weaponinfo_pickupammo _weaponinfo_equipmontage _weaponinfo_unequipmontage _weaponinfo_firemontage _weaponinfo_reloadmontage _weaponinfo_projectile _weaponinfo_muzzle) (break `/Game/BLUEPRINTS/ITEM_Pickups/Weapons/WeaponInfo` (`self.WeaponInfo`)))
  (set `self.WeaponInfo` (make `/Game/BLUEPRINTS/ITEM_Pickups/Weapons/WeaponInfo` _weaponinfo_weapontype (`GameplayStatics.GetObjectClass` self) _weaponinfo_name _weaponinfo_image _weaponinfo_equipsocket _weaponinfo_unequipsocket _weaponinfo_firerate _weaponinfo_damage _weaponinfo_range _weaponinfo_sound _weaponinfo_ammotype _weaponinfo_clipsize _weaponinfo_currentammo _weaponinfo_maxammo _weaponinfo_pickupammo _weaponinfo_equipmontage _weaponinfo_unequipmontage _weaponinfo_firemontage _weaponinfo_reloadmontage _weaponinfo_projectile _weaponinfo_muzzle)))