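; Level entry portal that loads a configured level when the DevatoxBP actor overlaps it, provided the portal is unlocked.
; Unlock state comes from comparing the drone save game's highest unlocked level to the portal's level, and sets the emissive material on the trim and base at BeginPlay.
; An unlocked overlap plays a sound and fade-to-black widget, then opens the level after a delay; a locked one only prints a message.
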(event `self.ReceiveBeginPlay`
  (bind _trim (`self.Trim`))
  (bind _returnvalue (`self.IsPortalUnlocked`))
  (if _returnvalue
    (`PrimitiveComponent.SetMaterial` _trim 1 "/Game/BLUEPRINTS/Materials/M_FloorOneEmissive.M_FloorOneEmissive")
    (`PrimitiveComponent.SetMaterial` (`self.Base`) 1 "/Game/BLUEPRINTS/Materials/M_FloorOneEmissive.M_FloorOneEmissive")
    (else
      (`PrimitiveComponent.SetMaterial` _trim 1 "/Game/BLUEPRINTS/Materials/M_FloorOneEmissiveTwo_Inst.M_FloorOneEmissiveTwo_Inst")
      (`PrimitiveComponent.SetMaterial` (`self.Base`) 1 "/Game/BLUEPRINTS/Materials/M_FloorOneEmissiveTwo_Inst.M_FloorOneEmissiveTwo_Inst"))))

(event `self.Overlap.OnComponentBeginOverlap`
  (params (OverlappedComponent :type "PrimitiveComponent Object Reference") (OtherActor :type "Actor Object Reference") (OtherComp :type "PrimitiveComponent Object Reference") (OtherBodyIndex :type Integer) (bFromSweep :type Boolean) (SweepResult :type "HitResult Structure (by ref)"))
  (cast `/Game/BLUEPRINTS/DevatoxBP` OtherActor)
  (bind _returnvalue (`self.IsPortalUnlocked`))
  (if _returnvalue
    (`GameplayStatics.SpawnSound2D` "/Game/BLUEPRINTS/Sounds/Interaction/CloseHUD.CloseHUD" 2.0 1.0 0.0 null)
    (bind _returnvalue_2 (`|CreateWidget` "/Game/BLUEPRINTS/UI/FadeToBlack.FadeToBlack_C"))
    (`/Game/BLUEPRINTS/UI/FadeToBlack.FadeToBlack` _returnvalue_2)
    (`UserWidget.AddToViewport` _returnvalue_2 0)
    (`KismetSystemLibrary.Delay` 3.0)
    (`GameplayStatics.OpenLevel` (`self.LevelToOpen`))
    (else
      (`KismetSystemLibrary.PrintString` "Level Not Unlocked"))))

(fn `IsPortalUnlocked`
  (returns (ReturnValue :type Boolean))
  (bind _asdrone_checkpont_save (`/Game/BLUEPRINTS/MyFunction.LoadDroneSaveGame`))
  (return (>= (`/Game/BLUEPRINTS/Interactables/Checkpoints/DroneCheckpont_Save.HighestLevelUnlocked` _asdrone_checkpont_save) (`self.PortalLevel`))))

(fn `UserConstructionScript`)