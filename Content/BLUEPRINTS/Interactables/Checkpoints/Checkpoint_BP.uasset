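; Checkpoint actor that saves the player's respawn point when DevatoxBP enters its sphere trigger.
; SaveGameData loads or creates a DroneCheckpont_Save, stores a transform raised above the checkpoint with reset rotation and scale, then writes it to the save slot.
; The overlap then shows a temporary "Game Saved Successful" popup with a 2D sound, removing the widget after a short delay.
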(event `self.Sphere.OnComponentBeginOverlap`
  (params (OverlappedComponent :type "PrimitiveComponent Object Reference") (OtherActor :type "Actor Object Reference") (OtherComp :type "PrimitiveComponent Object Reference") (OtherBodyIndex :type Integer) (bFromSweep :type Boolean) (SweepResult :type "HitResult Structure (by ref)"))
  (bind _returnvalue_location (`KismetMathLibrary.BreakTransform` (`self.GetTransform`)))
  (bind _asdevatox_bp (cast `/Game/BLUEPRINTS/DevatoxBP` OtherActor))
  (set `self.As Devatox BP` _asdevatox_bp)
  (bind _returnvalue (`GameplayStatics.DoesSaveGameExist` (`self.SaveName`)))
  (if _returnvalue
    (bind _returnvalue_2 (`GameplayStatics.LoadGameFromSlot` (`self.SaveName`)))
    (bind _asdrone_checkpont_save (cast `/Game/BLUEPRINTS/Interactables/Checkpoints/DroneCheckpont_Save` _returnvalue_2))
    (set `self.SaveGameREF` _asdrone_checkpont_save)
    (else
      (bind _returnvalue_3 (`GameplayStatics.CreateSaveGameObject` "/Game/BLUEPRINTS/Interactables/Checkpoints/DroneCheckpont_Save.DroneCheckpont_Save_C"))
      (set `self.SaveGameREF` _returnvalue_3)))
  (set `/Game/BLUEPRINTS/Interactables/Checkpoints/DroneCheckpont_Save.Checkpoint` (`KismetMathLibrary.MakeTransform` (+ _returnvalue_location (0.0 0.0 200.0))) (`self.SaveGameREF`))
  (`GameplayStatics.SaveGameToSlot` (`self.SaveGameREF`) (`self.SaveName`))
  (bind _returnvalue_4 (`|CreateWidget` "/Game/BLUEPRINTS/UI/PopupText.PopupText_C"))
  (`UserWidget.AddToViewport` _returnvalue_4 0)
  (`TextBlock.SetText` (`/Game/BLUEPRINTS/UI/PopupText.TextPopup` _returnvalue_4) "Game Saved Successful")
  (`GameplayStatics.SpawnSound2D` "/Game/BLUEPRINTS/Sounds/Interaction/OpenHUD.OpenHUD" 2.0 1.0 0.0 null)
  (`KismetSystemLibrary.Delay` 3.0)
  (`Widget.RemoveFromParent` _returnvalue_4))

(event `self.Sphere.OnComponentEndOverlap`
  (params (OverlappedComponent :type "PrimitiveComponent Object Reference") (OtherActor :type "Actor Object Reference") (OtherComp :type "PrimitiveComponent Object Reference") (OtherBodyIndex :type Integer)))

(fn `UserConstructionScript`)